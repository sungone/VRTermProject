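; BP_ButtonCubeManager pairs a button with a rotating-cube actor and links the two at runtime.
; On BeginPlay it casts its two Child Actor components to BP_Button and BP_RotCube and stores both references.
; It then passes the cube reference to the button, stopping early if either cast fails.
; It holds no interaction logic of its own, and its construction script is empty.
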(event EventBeginPlay
  (bind _asbp_button (Utilities|Casting|CastToBP_Button (Variables|/Script/Engine.ChildActorComponent|GetChildActor (Variables|Default|GetButtonChildActor))))
  (Variables|Default|SetButtonRef _asbp_button)
  (bind _asbp_rot_cube (Utilities|Casting|CastToBP_RotCube (Variables|/Script/Engine.ChildActorComponent|GetChildActor (Variables|Default|GetRotCubeChildActor))))
  (Variables|Default|SetRotCubeRef _asbp_rot_cube)
  (Variables|/Game/Team0/class/BP_Button.BP_Button_C|SetRotCubeRef (Variables|Default|GetButtonRef) (Variables|Default|GetRotCubeRef)))

(fn ConstructionScript)