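; BP_Probe is a grippable probe actor that shows its current rotation angle as text.
; The Axis setting orients the probe and its physics constraint at construction and selects whether pitch or yaw is displayed.
; Grip and release events toggle actor tick, so the clamped, two-decimal readout refreshes only while held.
; The text updates on remote clients or in standalone, skipping networked authority.
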(event EventBeginPlay
  (|CallParentFunction)
  (Variables|Default|SetInitRot (Variables|/Script/Engine.SceneComponent|GetRelativeRotation (Variables|Default|GetProbeComponent))))

(event EventTick
  (params (DeltaSeconds :type Float%20%28single-precision%29))
  (CallFunction|UpdateText))

(event EventOnChildGrip
  (params (GrippingController :type Grip%20Motion%20Controller%20Component%20Object%20Reference) (GripInformation :type BP%20Actor%20Grip%20Information%20Structure%20%28by%20ref%29))
  (Actor|Tick|SetActorTickEnabled true) ; The dial components tick is off
)

(event EventOnChildGripRelease
  (params (ReleasingController :type Grip%20Motion%20Controller%20Component%20Object%20Reference) (GripInformation :type BP%20Actor%20Grip%20Information%20Structure%20%28by%20ref%29) (bWasSocketed :type Boolean))
  (Actor|Tick|SetActorTickEnabled false))

(fn ConstructionScript
  (switch Utilities|FlowControl|Switch|SwitchonEVRInteractibleAxis (Variables|Default|GetAxis)
    (:Axis_X
      (Transformation|SetRelativeRotation (Variables|Default|GetProbeComponent) "0.000000,0.000000,-90.000000" false false))
    (:Axis_Y
      (Transformation|SetRelativeRotation (Variables|Default|GetProbeComponent) "0.000000,90.000000,-90.000000" false false))))

(fn UpdateText
  (bind _probecomponent (Variables|Default|GetProbeComponent))
  (bind _relativerotation (Variables|/Script/Engine.SceneComponent|GetRelativeRotation _probecomponent))
  (Networking|SwitchHasAuthority
    (:Authority
      (if (Class|KismetSystemLibrary|IsStandalone)
        (Rendering|Components|TextRender|SetText (Variables|Default|GetTextRender) (Utilities|Text|ToText(Float) (Class|KismetMathLibrary|ClampAxis (Utilities|Select :Index (Variables|Default|GetAxis) :Axis_X (.pitch _relativerotation) :Axis_Y (.pitch _relativerotation) :Axis_Z (.yaw _relativerotation))) "HalfToEven" false true 1 324 2 2) :!label _label)))
    (:Remote
      (goto _label))))