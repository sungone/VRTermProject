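; BP_LeverActor is a grippable lever that shows its current angle on a text display.
; It ticks only while gripped, refreshing the text on clients and in standalone games.
; On release, a dedicated server stores the final angle in LastAngle.
; Its OnRep handler applies that angle as the lever's roll, refreshes the text and prints debug output.
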(event OnDropped(LeverComponent)
  (params (GrippingController :type Grip%20Motion%20Controller%20Component%20Object%20Reference) (GripInformation :type BP%20Actor%20Grip%20Information%20Structure%20%28by%20ref%29) (bWasSocketed :type Boolean))
  (Actor|Tick|SetActorTickEnabled false)
  (if (Networking|IsDedicatedServer)
    (Variables|Default|SetLastAngle (.Actual%20Angle (Default|GetAngle (Variables|Default|GetLeverComponent))))))

(event OnGripped(LeverComponent)
  (params (GrippingController :type Grip%20Motion%20Controller%20Component%20Object%20Reference) (GripInformation :type BP%20Actor%20Grip%20Information%20Structure%20%28by%20ref%29))
  (Actor|Tick|SetActorTickEnabled true))

(event EventTick
  (params (DeltaSeconds :type Float%20%28single-precision%29))
  (CallFunction|UpdateAngleText))

(fn ConstructionScript)

(fn UpdateAngleText
  (Networking|SwitchHasAuthority
    (:Authority
      (if (Class|KismetSystemLibrary|IsStandalone)
        (Rendering|Components|TextRender|SetText (Variables|Default|GetAngle) (Utilities|Text|ToText(Float) (.Actual%20Angle (Default|GetAngle (Variables|Default|GetLeverComponent))) "ToZero" false true 2 324 1 1) :!label _label)))
    (:Remote
      (goto _label))))

(fn OnRepLastAngle
  (bind _levercomponent (Variables|Default|GetLeverComponent))
  (bind _relativerotation (Variables|/Script/Engine.SceneComponent|GetRelativeRotation _levercomponent))
  (Transformation|SetRelativeRotation _levercomponent (Math|Rotator|MakeRotator (Variables|Default|GetLastAngle) (.pitch _relativerotation) (.yaw _relativerotation)) false false)
  (CallFunction|UpdateAngleText)
  (Development|PrintString (Utilities|String|Append (Utilities|String|ToString(Float) (Variables|Default|GetLastAngle)) " / " (Utilities|String|ToString(Rotator) (Variables|/Script/Engine.SceneComponent|GetRelativeRotation _levercomponent)))))