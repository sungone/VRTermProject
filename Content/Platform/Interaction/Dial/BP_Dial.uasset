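; BP_Dial is a grippable VR dial that displays its current angle as text.
; The construction script orients the dial and physics constraint to the chosen axis.
; Actor tick runs from grip to release, refreshing the text on remote clients or in standalone.
; On release, a dedicated server stores the final angle, reapplies it without events, and the variable's RepNotify refreshes the text.
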(event EventBeginPlay
  (|CallParentFunction))

(event EventTick
  (params (DeltaSeconds :type Float%20%28single-precision%29))
  (CallFunction|UpdateText))

(event EventOnChildGrip
  (params (GrippingController :type Grip%20Motion%20Controller%20Component%20Object%20Reference) (GripInformation :type BP%20Actor%20Grip%20Information%20Structure%20%28by%20ref%29))
  (Variables|Default|SetGripping%20Controller GrippingController)
  (Actor|Tick|SetActorTickEnabled true) ; The dial components tick is off
)

(event EventOnChildGripRelease
  (params (ReleasingController :type Grip%20Motion%20Controller%20Component%20Object%20Reference) (GripInformation :type BP%20Actor%20Grip%20Information%20Structure%20%28by%20ref%29) (bWasSocketed :type Boolean))
  (bind _vrdial (Variables|Default|GetVRDial))
  (Actor|Tick|SetActorTickEnabled false)
  (if (Networking|IsDedicatedServer)
    (bind _output_get (Variables|Default|SetLasted%20Dial%20Angle (Variables|/Script/VRExpansionPlugin.VRDialComponent|GetCurrentDialAngle _vrdial)))
    (Class|VRDialComponent|SetDialAngle _vrdial _output_get false)))

(fn ConstructionScript
  (switch Utilities|FlowControl|Switch|SwitchonEVRInteractibleAxis (Variables|Default|GetAxis)
    (:Axis_X
      (Transformation|SetRelativeRotation (Variables|Default|GetPhysicsConstraint) "0.000000,90.000000,0.000000" false false)
      (Transformation|SetRelativeRotation (Variables|Default|GetVRDial) "0.000000,90.000000,0.000000" false false))
    (:Axis_Z
      (Transformation|SetRelativeRotation (Variables|Default|GetPhysicsConstraint) "0.000000,0.000000,-90.000000" false false)
      (Transformation|SetRelativeRotation (Variables|Default|GetVRDial) "0.000000,0.000000,-90.000000" false false))))

(fn UpdateText
  (Networking|SwitchHasAuthority
    (:Authority
      (if (Class|KismetSystemLibrary|IsStandalone)
        (Rendering|Components|TextRender|SetText (Variables|Default|GetTextRender) (Utilities|Text|ToText(Float) (Variables|/Script/VRExpansionPlugin.VRDialComponent|GetCurrentDialAngle (Variables|Default|GetVRDial)) "HalfToEven" false true 1 324 2 2) :!label _label)))
    (:Remote
      (goto _label))))

(fn OnRepLastedDialAngle
  (CallFunction|UpdateText))