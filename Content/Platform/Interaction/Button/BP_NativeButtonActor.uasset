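; BP_NativeButtonActor is an interactive button actor that shows On or Off text matching its button component's state.
; The text refreshes on BeginPlay and whenever ButtonComp reports a state change, updating only on remote instances or in standalone games.
; A LastButtonState RepNotify syncs the component without re-firing its change event, then updates the text and button color.
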(event OnButtonStateChanged(ButtonComp)
  (params (ButtonState :type Boolean) (InteractingActor :type Actor%20Object%20Reference) (InteractingComponent :type Primitive%20Component%20Object%20Reference))
  (CallFunction|SetText ButtonState))

(event Custom|SetText
  (params (State :type Boolean))
  (bind _textrender (Variables|Components|GetTextRender))
  (Networking|SwitchHasAuthority
    (:Authority
      (if (Class|KismetSystemLibrary|IsStandalone)
        (if State :!label _label
          (Rendering|Components|TextRender|SetText _textrender (Variables|Default|GetOnText))
          (else
            (Rendering|Components|TextRender|SetText _textrender (Variables|Default|GetOffText))))))
    (:Remote
      (goto _label))))

(event EventBeginPlay
  (CallFunction|SetText (Variables|/Script/VRExpansionPlugin.VRButtonComponent|GetbButtonState (Variables|Default|GetButtonComp))))

(fn ConstructionScript)

(fn OnRepLastButtonState
  (bind _lastbuttonstate (Variables|Default|GetLastButtonState))
  (bind _buttoncomp (Variables|Default|GetButtonComp))
  (Class|VRButtonComponent|SetButtonState _buttoncomp _lastbuttonstate false false)
  (CallFunction|SetText _lastbuttonstate)
  (Default|SetColor _buttoncomp))