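; Networked VR slider actor that players grip and slide, displaying its axis and current progress as text.
; At BeginPlay, Init infers the axis from the first non-zero slide limit, orients the components to suit and labels the axis on clients.
; Gripping enables Tick to refresh the value text on clients or standalone, and dropping disables it.
; On drop, a dedicated server stores progress in LastSliderProgress, whose OnRep repositions the slider and updates the text.
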(event OnDropped(VRSlider)
  (params (GrippingController :type Grip%20Motion%20Controller%20Component%20Object%20Reference) (GripInformation :type BP%20Actor%20Grip%20Information%20Structure%20%28by%20ref%29) (bWasSocketed :type Boolean))
  (Actor|Tick|SetActorTickEnabled false)
  (if (Networking|IsDedicatedServer)
    (Variables|Default|SetLastSliderProgress (Variables|/Script/VRExpansionPlugin.VRSliderComponent|GetCurrentSliderProgress (Variables|Default|GetVRSlider)))))

(event OnGripped(VRSlider)
  (params (GrippingController :type Grip%20Motion%20Controller%20Component%20Object%20Reference) (GripInformation :type BP%20Actor%20Grip%20Information%20Structure%20%28by%20ref%29))
  (Actor|Tick|SetActorTickEnabled true))

(event EventBeginPlay
  (CallFunction|Init (Variables|Default|GetVRSlider)))

(event EventTick
  (params (DeltaSeconds :type Float%20%28single-precision%29))
  (CallFunction|UpdateValue))

(fn ConstructionScript)

(fn UpdateValue
  (Networking|SwitchHasAuthority
    (:Authority
      (if (Class|KismetSystemLibrary|IsStandalone)
        (Rendering|Components|TextRender|SetText (Variables|Default|GetValueText) (Utilities|Text|ToText(Float) (Variables|/Script/VRExpansionPlugin.VRSliderComponent|GetCurrentSliderProgress (Variables|Default|GetVRSlider)) "HalfToEven") :!label _label)))
    (:Remote
      (goto _label))))

(fn OnRepLastSliderProgress
  (Class|VRSliderComponent|SetSliderProgress (Variables|Default|GetVRSlider) (Variables|Default|GetLastSliderProgress))
  (CallFunction|UpdateValue))

(fn Init
  (params (Slider :type VR%20Slider%20Component%20Object%20Reference))
  (bind _minslidedistance (Variables|/Script/VRExpansionPlugin.VRSliderComponent|GetMinSlideDistance Slider))
  (bind _maxslidedistance (Variables|/Script/VRExpansionPlugin.VRSliderComponent|GetMaxSlideDistance Slider))
  (if (or (!= (.x _maxslidedistance) 0.0) (!= (.x _minslidedistance) 0.0))
    (Variables|Default|SetAxis "Axis_X")
    (Transformation|SetRelativeRotation (Variables|Default|GetStaticMesh) "0.000000,90.000000,0.000000" false false)
    (Networking|SwitchHasAuthority
      (:Remote
        (Rendering|Components|TextRender|SetText (Variables|Default|GetAxisText) (Utilities|Text|MakeLiteralText "X"))))
    (elif (or (!= (.y _maxslidedistance) 0.0) (!= (.y _minslidedistance) 0.0))
      (Variables|Default|SetAxis "Axis_Y")
      (Networking|SwitchHasAuthority
        (:Remote
          (Rendering|Components|TextRender|SetText (Variables|Default|GetAxisText) (Utilities|Text|MakeLiteralText "Y"))))
      (elif (or (!= (.z _maxslidedistance) 0.0) (!= (.z _minslidedistance) 0.0))
        (Variables|Default|SetAxis "Axis_Z")
        (Transformation|SetRelativeRotation (Variables|Default|GetStaticMesh) "0.000000,-90.000000,90.000000" false false)
        (Transformation|SetRelativeRotation (Variables|Default|GetVRSlider) "-90.000000,0.000000,0.000000" false false)
        (Networking|SwitchHasAuthority
          (:Remote
            (Rendering|Components|TextRender|SetText (Variables|Default|GetAxisText) (Utilities|Text|MakeLiteralText "Z"))))
        (else
          (Networking|SwitchHasAuthority
            (:Remote
              (Rendering|Components|TextRender|SetText (Variables|Default|GetAxisText) (Utilities|Text|MakeLiteralText "None")))))))))