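; Shooting effect actor that plays a configurable Niagara effect carried by a projectile movement component.
; The construction script assigns the Niagara asset and offsets the effect along world X by Speed.
; On BeginPlay it moves root and effect to InitialPos and activates effect and movement.
; A non-looping timer applies one more X offset at three seconds, then effect and movement deactivate half a second later, without destroying the actor.
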(event Custom|Move
  (bind _e (Variables|Default|Gete))
  (bind _returnvalue (Transformation|GetWorldLocation _e))
  (Transformation|SetWorldLocation _e (Math|Vector|MakeVector (+ (.x _returnvalue) (Variables|Default|GetSpeed)) (.y _returnvalue) (.z _returnvalue)) false false))

(event EventBeginPlay
  (Transformation|SetWorldLocation (Variables|Default|GetDefaultSceneRoot) (Variables|Default|GetInitialPos) false false)
  (Components|Activation|SetActive (Variables|Default|Gete) true true)
  (bind _returnvalue (Utilities|Time|SetTimerbyEvent (delegate Custom|Move) 3.0))
  (Utilities|FlowControl|Delay 3.5)
  (Components|Activation|Deactivate (Variables|Default|Gete))
  (Components|Activation|SetActive (Variables|Default|GetProjectileMovement) false false)
  (Utilities|Time|ClearandInvalidateTimerbyHandle _returnvalue))

(fn ConstructionScript
  (bind _e (Variables|Default|Gete))
  (bind _returnvalue (Transformation|GetWorldLocation _e))
  (Class|NiagaraComponent|SetAsset (Variables|Default|Gete) (Variables|Default|GetNiagara) true)
  (Transformation|SetWorldLocation (Variables|Default|Gete) (Math|Vector|MakeVector (+ (.x _returnvalue) (Variables|Default|GetSpeed)) (.y _returnvalue) (.z _returnvalue)) false false))