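; Base HUD Blueprint for the shooting game that organizes widget setup into four categories.
; BeginPlay passes the player controller to InitGame, InitGameMenu, InitMenu and InitModals in turn.
; These are meant for always-on widgets, toggleable in-game widgets, out-of-game menus such as login, and popups or notifications.
; All four functions are empty scaffolding here, so no widgets are created yet.
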(event EventBeginPlay
  (bind _returnvalue (Game|GetPlayerController 0))
  (Initialize|InitGame _returnvalue) ; Always On Display
  (Initialize|InitGameMenu _returnvalue) ; In-game Widget
  (Initialize|InitMenu _returnvalue) ; Out Menu WIdget
  (Initialize|InitModals _returnvalue) ; Pop-up Widget
)

(fn ConstructionScript)

(fn InitGame
  (params (PlayerController :type Player%20Controller%20Object%20Reference))
  (Utilities|FlowControl|Sequence))

(fn InitGameMenu
  (params (PlayerController :type Player%20Controller%20Object%20Reference))
  (Utilities|FlowControl|Sequence))

(fn InitMenu
  (params (PlayerController :type Player%20Controller%20Object%20Reference))
  (Utilities|FlowControl|Sequence))

(fn InitModals
  (params (PlayerController :type Player%20Controller%20Object%20Reference)))