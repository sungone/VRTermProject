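; BP_Pistol is a pistol actor that fires a line trace when key 3 is pressed and reports target hits to a monitor.
; The trace starts at its Arrow component and ends at the scaled forward vector, without adding the start location.
; Hits on BP_Target get a hardcoded offset, then their X and Z go to BP_Monitor's ShotOfBPMonitor.
; Persistent trace drawing and printed messages provide debug output.
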(event EventBeginPlay
  ;[0.15 0.15 0.15 0.5] Enable Input
  (Input|EnableInput (Game|GetPlayerController 0)))

(event Collision|EventActorBeginOverlap
  (params (OtherActor :type Actor%20Object%20Reference)))

(event EventTick
  (params (DeltaSeconds :type Float%20%28single-precision%29)))

(event Input|KeyboardEvents|3
  (params (Key :type Key%20Structure :default "None"))
  (:Pressed
    (Development|PrintString "Shoot")
    (bind _outhit (Collision|LineTraceByChannel (Transformation|GetWorldLocation (Variables|Default|GetArrow)) (* (Math|Vector|GetForwardVector (Variables|Default|GetArrow)) 1e+03) "TraceTypeQuery4" false 0 "Persistent"))
    (Utilities|Casting|CastToBP_Target (.HitActor (Collision|BreakHitResult _outhit)))
    (Variables|Default|SetShoot%20Point (.ImpactPoint (Collision|BreakHitResult _outhit)))
    (bind _output_get (Variables|Default|SetReal%20Shoot%20Point (+ (Variables|Default|GetShoot%20Point) "83.000000,0.000000,-157.000000")))
    (Development|PrintString (Utilities|String|ToString(Vector) _output_get) true true "(R=0.279944,G=1.000000,B=0.223156,A=1.000000)" 5e+01)
    (bind _returnvalue (Actor|GetActorOfClass "/Game/Shooting/UI/BP_Monitor.BP_Monitor_C"))
    (Default|ShotOfBPMonitor _returnvalue (.x (Variables|Default|GetReal%20Shoot%20Point)) (.z (Variables|Default|GetReal%20Shoot%20Point)))))

(fn ConstructionScript)