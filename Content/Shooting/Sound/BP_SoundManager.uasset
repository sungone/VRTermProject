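; BP_SoundManager plays the audio for the shooting game: gunshots, score-based crowd applause and crowd ambience.
; BeginPlay starts a looping crowd noise as 2D sound, and SoundShot plays an air pistol shot at a given location.
; SoundApplause maps a 0–10 score to tiered applause or cheer sounds, then plays the chosen one at three world sound-location components.
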(event EventBeginPlay
  (CallFunction|SoundCrowdNoise))

(event Collision|EventActorBeginOverlap
  (params (OtherActor :type Actor%20Object%20Reference)))

(event EventTick
  (params (DeltaSeconds :type Float%20%28single-precision%29)))

(fn ConstructionScript)

(fn SoundShot
  (params (Loc :type Vector))
  (Audio|PlaySoundatLocation "/Game/Shooting/Sound/Sounds/air_pistol_one_shot.air_pistol_one_shot" Loc "0, 0, 0" 1.0 1.0 0.0 0 0 0 0))

(fn SoundApplause
  (params (Score%20Amount :type Integer))
  (switch int Score%20Amount
    (:0
      (Variables|Default|SetApplauseSound "/Game/Shooting/Sound/Sounds/Lv1_applause.Lv1_applause" :!label _label))
    (:1
      (goto _label))
    (:2
      (Variables|Default|SetApplauseSound "/Game/Shooting/Sound/Sounds/Lv2_applause.Lv2_applause" :!label _label_2))
    (:3
      (goto _label_2))
    (:4
      (Variables|Default|SetApplauseSound "/Game/Shooting/Sound/Sounds/Lv3_applause1.Lv3_applause1" :!label _label_3))
    (:5
      (goto _label_3))
    (:6
      (Variables|Default|SetApplauseSound "/Game/Shooting/Sound/Sounds/Lv3_applause2.Lv3_applause2" :!label _label_4))
    (:7
      (goto _label_4))
    (:8
      (Variables|Default|SetApplauseSound "/Game/Shooting/Sound/Sounds/Lv4_crowd-cheer.Lv4_crowd-cheer" :!label _label_5))
    (:9
      (goto _label_5))
    (:10
      (Variables|Default|SetApplauseSound "/Game/Shooting/Sound/Sounds/Lv5_crowd-cheers.Lv5_crowd-cheers")))
  (Utilities|FlowControl|Sequence
    (:then_0
      (Audio|PlaySoundatLocation (Variables|Default|GetApplauseSound) (Transformation|GetWorldLocation (Variables|Default|GetSound%20Location%201)) "0, 0, 0" 1.0 1.0 0.0 0 0 0 0))
    (:then_1
      (Audio|PlaySoundatLocation (Variables|Default|GetApplauseSound) (Transformation|GetWorldLocation (Variables|Default|GetSound%20Location%202)) "0, 0, 0" 1.0 1.0 0.0 0 0 0 0))
    (:then_2
      (Audio|PlaySoundatLocation (Variables|Default|GetApplauseSound) (Transformation|GetWorldLocation (Variables|Default|GetSound%20Location%203)) "0, 0, 0" 1.0 1.0 0.0 0 0 0 0))))

(fn SoundCrowdNoise
  (Audio|PlaySound2D "/Game/Shooting/Sound/Sounds/loop_crowd_noise.loop_crowd_noise" 1.0 1.0 0.0 0 0))