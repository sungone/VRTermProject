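; AI shooter character that holds a pistol on a mesh socket and fires repeatedly at random intervals, up to a shot cap.
; ShotAnim plays a montage, whose "Shoot" notify triggers the gunshot sound and spawns BP_ShootEffect at the socket.
; Montage completion schedules the next shot by timer.
; Init resets the counter and restarts firing after a random delay, while NotifyEnding clears the ready flag that gates firing.
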(event Custom|Shot%20Anim
  (bind _mesh (Variables|Character|GetMesh))
  (bind _returnvalue (Transformation|GetSocketLocation _mesh "PistolSocket"))
  (if (and (Variables|Default|GetAnimReady) (< (Variables|Default|GetShootCount) 60))
    (Variables|Default|SetAnimReady false)
    (Variables|Default|SetShootCount (+ (Variables|Default|GetShootCount) 1))
    (bind _notifyname (Animation|Montage|PlayMontage (Variables|Character|GetMesh) "/Game/Shooting/AI/AM_AICharacter.AM_AICharacter")
      (:OnCompleted
        (Variables|Default|SetAnimReady true)
        (bind _output_get (Variables|Default|SetRandSec (Math|Random|RandomFloatinRange 4.0 7.0)))
        (Utilities|Time|SetTimerbyEvent (delegate Custom|Shot%20Anim) _output_get))
      (:OnNotifyBegin
        (if (== _notifyname "Shoot")
          (Audio|PlaySoundatLocation "/Game/Shooting/Sound/Sounds/air_pistol_one_shot.air_pistol_one_shot" _returnvalue "0, 0, 0" (Math|Float|MakeLiteralFloat 0.8) 1.0 0.0 0 0 0 0)
          (Game|SpawnActorfromClass "/Game/Shooting/BP_ShootEffect.BP_ShootEffect_C" (Math|Transform|MakeTransform _returnvalue "0.000000,90.000000,0.000000" "0.100000,0.100000,0.100000") "Undefined" "MultiplyWithRoot" 0 3e+04 _returnvalue 0))))))

(event Custom|Init
  (Variables|Default|SetShootCount 0)
  (Variables|Default|SetAnimReady true)
  (Utilities|FlowControl|Delay (Math|Random|RandomFloatinRange 0.0 2.0))
  (CallFunction|ShotAnim))

(event EventBeginPlay
  (Variables|Default|SetShootCount 0)
  (Variables|Default|SetAnimReady true)
  (Transformation|AttachComponentToComponent (Variables|Default|GetPistol) (Variables|Character|GetMesh) "PistolSocket" "SnapToTarget" "SnapToTarget" "SnapToTarget" true)
  (Utilities|FlowControl|Delay (Math|Random|RandomFloatinRange 0.0 2.0))
  (CallFunction|ShotAnim))

(event Collision|EventActorBeginOverlap
  (params (OtherActor :type Actor%20Object%20Reference)))

(event EventTick
  (params (DeltaSeconds :type Float%20%28single-precision%29)))

(event EventNotifyEnding
  (Variables|Default|SetAnimReady false))

(fn ConstructionScript)